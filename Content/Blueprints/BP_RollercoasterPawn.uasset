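; BP_RollercoasterPawn is the rollercoaster pawn Blueprint that handles ride audio for the track and the climbing gears.
; Events for climbing, falling, fading and stopping crossfade or fade out TrackSound and GearsSound.
; Every tick it reads the current coaster velocity from the RollercoasterPlayerController and feeds it into TrackSound's Speed parameter, so the track audio follows the ride speed.
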(event `FadeTrackSound`
  (`AudioComponent.FadeOut` (`self.TrackSound`) 3.0 0.0 :!label _label))

(event `StartClimbing`
  (`AudioComponent.FadeIn` (`self.GearsSound`) 6.0 1.0 0.0)
  (goto _label))

(event `StartFalling`
  (`AudioComponent.FadeIn` (`self.TrackSound`) 3.0 1.0 0.0)
  (`AudioComponent.FadeOut` (`self.GearsSound`) 1.0 0.0))

(event `StopTrackSound`
  (`AudioComponent.FadeOut` (`self.TrackSound`) 0.5 0.0))

(event `self.ReceiveTick`
  (params (DeltaSeconds :type "Float (single-precision)"))
  (bind _asrollercoaster_player_controller (cast `RollercoasterPlayerController` (`GameplayStatics.GetPlayerController` 0)))
  (`AudioComponent.SetFloatParameter` (`self.TrackSound`) "Speed" (`RollercoasterPlayerController.CurrentRollerCoasterVelocity` _asrollercoaster_player_controller)))

(fn `UserConstructionScript`)