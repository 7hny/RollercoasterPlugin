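; Player controller for a rollercoaster game that relays input and climb or fall state changes to the rollercoaster pawn.
; It caches the pawn on BeginPlay; touch or Enter clears the stopped flag, hides the pawn's text and HUD, and starts climbing.
; Custom events also trigger climbing, or switch to falling while clearing the climb flag and added velocity.
; Escape quits the game.
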(event `self.ReceiveBeginPlay`
  (bind _asbp_rollercoaster_pawn (cast `/RollercoasterPlugin/Blueprints/BP_RollercoasterPawn` (`GameplayStatics.GetPlayerPawn` 0)))
  (set `self.PlayerPawn` _asbp_rollercoaster_pawn))

(event `InputTouch`
  (params (Location :type "Object.Vector Structure") (FingerIndex :type "InputCoreTypes.ETouchIndex Enum"))
  (:`Pressed`
    (set `self.Stopped` false :!label _label)
    (`SceneComponent.SetHiddenInGame` (`/RollercoasterPlugin/Blueprints/BP_RollercoasterPawn.TextRender` (`self.PlayerPawn`)) true true :!label _label_2)
    (`SceneComponent.SetHiddenInGame` (`/RollercoasterPlugin/Blueprints/BP_RollercoasterPawn.HudContainer` (`self.PlayerPawn`)) true true)
    (set `self.Climbing` true)
    (`/RollercoasterPlugin/Blueprints/BP_RollercoasterPawn.StartClimbing` (`self.PlayerPawn`))))

(event `Key|Enter`
  (:`Pressed`
    (goto _label)))

(event `EventStartClimbing`
  (goto _label_2))

(event `EventStartFalling`
  (`/RollercoasterPlugin/Blueprints/BP_RollercoasterPawn.StartFalling` (`self.PlayerPawn`))
  (set `self.Climbing` false)
  (set `self.AddVelocity` 0.0))

(event `Key|Escape`
  (:`Pressed`
    (`KismetSystemLibrary.QuitGame` null "Quit")))

(fn `UserConstructionScript`)